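; BP_statusEffects is a timed status effect that belongs to an owning actor, with an empty tick event as a placeholder for effect behavior.
; Attempt starts two timers from StatusEffectInfo: a looping tick at TickTime and an end timer after Length.
; On expiry, it clears both timers and calls RemoveStatusEffects on the owner's AC_StatusEffects component, if one exists.
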(event Custom|Attempt
  (CallFunction|StartStatusEffect))

(event Custom|StartStatusEffect
  (bind _statuseffectinfo (Variables|Default|GetStatusEffectInfo))
  (bind (_length _ticktime) (Utilities|Struct|BreakS_StatusEffects _statuseffectinfo))
  (bind _returnvalue (Utilities|Time|SetTimerbyEvent (delegate Custom|TickEvent) _ticktime true))
  (Variables|Default|SetTickTimerHandle _returnvalue)
  (bind _returnvalue_2 (Utilities|Time|SetTimerbyEvent (delegate Custom|EndStatusEffect) _length false false 0.001))
  (Variables|Default|SetLengthTimerHandle _returnvalue_2))

(event Custom|TickEvent)

(event Custom|EndStatusEffect
  (bind _returnvalue (Components|GetOwner))
  (bind _returnvalue_2 (Actor|GetComponentbyClass _returnvalue "/Game/Status_Effects/AC_StatusEffects.AC_StatusEffects_C"))
  ;[1 1 1] Ending Effect
  ;;[1 1 1] Clears the timers
  (CallFunction|ClearTImers)
  (Utilities|IsValid _returnvalue_2
    (:Is%20Valid
      (Default|RemoveStatusEffects _returnvalue_2 (Variables|Default|GetReplaceWithSelf)))))

(fn ConstructionScript)

(fn ClearTImers
  (Utilities|Time|ClearandInvalidateTimerbyHandle (Variables|Default|GetTickTimerHandle))
  (Utilities|Time|ClearandInvalidateTimerbyHandle (Variables|Default|GetLengthTimerHandle)))