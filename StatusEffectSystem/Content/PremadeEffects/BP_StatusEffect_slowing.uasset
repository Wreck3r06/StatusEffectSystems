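; Status effect Blueprint that temporarily slows the actor that owns it.
; On start, it sets the owner's CharacterMovementComponent MaxWalkSpeed to half of PreviousWalkSpeed and starts a timer using the length from StatusEffectInfo.
; When the timer fires, EndStatusEffect restores PreviousWalkSpeed and deactivates the SlowingEffect component.
; PreviousWalkSpeed is only read in these graphs, never captured from the owner.
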(event EventStartStatusEffect
  (bind _returnvalue (Components|GetOwner))
  (bind _returnvalue_2 (Actor|GetComponentbyClass _returnvalue "/Script/Engine.CharacterMovementComponent"))
  ;[0.0731 0.8073 0] Start Slowing Effect
  (Utilities|IsValid _returnvalue_2
    (:Is%20Valid
      ;;[1 1 1] Calculations for speed
      (Variables|/Script/Engine.CharacterMovementComponent|SetMaxWalkSpeed _returnvalue_2 (/ (Variables|Default|GetPreviousWalkSpeed) 2.0))
      (Utilities|Time|SetTimerbyEvent (delegate EventEndStatusEffect) (.Length (Utilities|Struct|BreakS_StatusEffects (Variables|Default|GetStatus%20Effect%20Info)))))))

(event EventEndStatusEffect
  (bind _returnvalue (Components|GetOwner))
  (bind _returnvalue_2 (Actor|GetComponentbyClass _returnvalue "/Script/Engine.CharacterMovementComponent"))
  ;[1 0 0] End Slowing Effect
  (Utilities|IsValid _returnvalue_2
    (:Is%20Valid
      (Variables|/Script/Engine.CharacterMovementComponent|SetMaxWalkSpeed _returnvalue_2 (Variables|Default|GetPreviousWalkSpeed))
      (Components|Activation|Deactivate (Variables|Default|GetSlowingEffect)))))

(fn ConstructionScript
  (|CallParentFunction))