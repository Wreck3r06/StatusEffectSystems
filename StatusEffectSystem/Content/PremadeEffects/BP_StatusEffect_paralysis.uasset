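; Paralysis status effect Blueprint that freezes its owning character's movement for a limited time.
; On start it sets the owner's CharacterMovementComponent movement mode to None and sets a timer using the Length from StatusEffectInfo.
; When the timer fires, it restores Walking mode and deactivates the Paralysis component.
; Both steps act only if the owner has a valid CharacterMovementComponent.
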(event EventStartStatusEffect
  (bind _returnvalue (Components|GetOwner))
  (bind _returnvalue_2 (Actor|GetComponentbyClass _returnvalue "/Script/Engine.CharacterMovementComponent"))
  ;[0.09291 0.4948 0] Start Satus Effect
  (Utilities|IsValid _returnvalue_2
    (:Is%20Valid
      (Pawn|Components|CharacterMovement|SetMovementMode _returnvalue_2 "MOVE_None" 0)
      (Utilities|Time|SetTimerbyEvent (delegate EventEndStatusEffect) (.Length (Utilities|Struct|BreakS_StatusEffects (Variables|Default|GetStatus%20Effect%20Info)))))))

(event EventEndStatusEffect
  (bind _returnvalue (Components|GetOwner))
  (bind _returnvalue_2 (Actor|GetComponentbyClass _returnvalue "/Script/Engine.CharacterMovementComponent"))
  ;[0.9219 0 0.08047] Ending Status Effect
  (Utilities|IsValid _returnvalue_2
    (:Is%20Valid
      (Pawn|Components|CharacterMovement|SetMovementMode _returnvalue_2 "MOVE_Walking" 0)
      (Components|Activation|Deactivate (Variables|Default|GetParalysis)))))

(fn ConstructionScript
  (|CallParentFunction))