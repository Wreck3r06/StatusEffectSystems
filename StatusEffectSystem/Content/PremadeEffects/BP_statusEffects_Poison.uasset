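; Premade poison status effect template that applies repeating fixed damage to a placeholder HP variable, meant to be swapped for the character's own HP.
; On start, it checks the owner for a generic component, then sets a looping damage timer and an end timer from StatusEffectInfo.
; Ending only zeroes TickDamage; the looping timer is never cleared, and each tick resets the damage before applying it.
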(event Custom|Damage%20Done
  (Variables|Default|SetTickDamage 3.0)
  (Variables|Default|SetHP (- (Variables|Default|GetHP) (Variables|Default|GetTickDamage))))

(event EventStartStatusEffect
  (bind _status_effect_info (Variables|Default|GetStatus%20Effect%20Info))
  (bind (_length _ticktime) (Utilities|Struct|BreakS_StatusEffects _status_effect_info))
  (Utilities|IsValid (Actor|GetComponentbyClass (Components|GetOwner) "/Script/Engine.ActorComponent")
    (:Is%20Valid
      (Utilities|Time|SetTimerbyEvent (delegate Custom|Damage%20Done) _ticktime true)
      (Utilities|Time|SetTimerbyEvent (delegate EventEndStatusEffect) _length))))

(event EventEndStatusEffect
  (Utilities|IsValid (Actor|GetComponentbyClass (Components|GetOwner) "/Script/Engine.ActorComponent")
    (:Is%20Valid
      (Variables|Default|SetTickDamage 0.0))))

(fn ConstructionScript
  (|CallParentFunction))