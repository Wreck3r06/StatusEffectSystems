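; BP_statusEffects_Vision is a timed status effect that alters vision through a PostProcess component.
; On start, if its owner is valid, it activates the PostProcess and sets both its lifespan and an end timer from StatusEffectInfo.Length.
; The end event deactivates the PostProcess if the owner is still valid.
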(event EventStartStatusEffect
  (bind _status_effect_info (Variables|Default|GetStatus%20Effect%20Info))
  (bind _length (Utilities|Struct|BreakS_StatusEffects _status_effect_info))
  ;[0.02344 0.5521 0.03005] Start Status effect
  (Utilities|IsValid (Components|GetOwner)
    (:Is%20Valid
      (Components|Activation|Activate (Variables|Default|GetPostProcess) false)
      ;;[1 1 1] How long the effect will last
      (Actor|SetLifeSpan _length)
      (Utilities|Time|SetTimerbyEvent (delegate EventEndStatusEffect) _length))))

(event EventEndStatusEffect
  ;[1 0 0] End Status effect
  (Utilities|IsValid (Components|GetOwner)
    (:Is%20Valid
      (Components|Activation|Deactivate (Variables|Default|GetPostProcess)))))

(fn ConstructionScript
  (|CallParentFunction))