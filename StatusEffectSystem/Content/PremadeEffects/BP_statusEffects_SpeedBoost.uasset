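; BP_statusEffects_SpeedBoost is a premade status effect that temporarily raises its owner's walk speed.
; On start it sets the owner's CharacterMovementComponent MaxWalkSpeed to the stored previous speed times a boost multiplier.
; A timer lasting the status effect's configured length then restores the previous speed and deactivates the boost effect.
; PrevMaxSpeed is only read in these graphs, never captured.
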(event EventEndStatusEffect
  (bind _returnvalue (Components|GetOwner))
  (bind _returnvalue_2 (Actor|GetComponentbyClass _returnvalue "/Script/Engine.CharacterMovementComponent"))
  ;[1 0 0] Ending effect
  (Utilities|IsValid _returnvalue_2
    (:Is%20Valid
      (Variables|/Script/Engine.CharacterMovementComponent|SetMaxWalkSpeed _returnvalue_2 (Variables|Default|GetPrevMaxSpeed))
      (Components|Activation|Deactivate (Variables|Default|GetSpeedBoostEffect)))))

(event EventStartStatusEffect
  (bind _returnvalue (Components|GetOwner))
  (bind _returnvalue_2 (Actor|GetComponentbyClass _returnvalue "/Script/Engine.CharacterMovementComponent"))
  ;[0 0.8906 0.1154] Starts the effect
  (Utilities|IsValid _returnvalue_2
    (:Is%20Valid
      ;;[1 1 1] Calculations
      (Variables|/Script/Engine.CharacterMovementComponent|SetMaxWalkSpeed _returnvalue_2 (* (Variables|Default|GetPrevMaxSpeed) (Variables|Default|GetSpeedBoost)))
      (Utilities|Time|SetTimerbyEvent (delegate EventEndStatusEffect) (.Length (Utilities|Struct|BreakS_StatusEffects (Variables|Default|GetStatus%20effect%20info)))))))

(fn ConstructionScript
  (|CallParentFunction))